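; A locked level-exit door behind glass, opened by two pressure plates that react to the third-person character.
; The first plate hides two SuperGridPlane panels and disables their collision.
; The second plate sets DoorUnlocked, after which overlapping the door trigger loads TargetLevelName.
; Both plates share one PressurePlatePressed flag, set just before it is checked, so neither depends on the other in logic.
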(event OnComponentBeginOverlap(Box2)
  (params (OverlappedComponent :type Primitive%20Component%20Object%20Reference) (OtherActor :type Actor%20Object%20Reference) (OtherComp :type Primitive%20Component%20Object%20Reference) (OtherBodyIndex :type Integer) (bFromSweep :type Boolean) (SweepResult :type Hit%20Result%20Structure%20%28by%20ref%29))
  ;[1 1 1] Pressure Plate 2
  (Utilities|Casting|CastToBP_ThirdPersonCharacter OtherActor)
  (Variables|Default|SetPressure%20Plate%20Pressed true)
  (if (Variables|Default|GetPressure%20Plate%20Pressed)
    (Variables|Default|SetDoor%20Unlocked true)))

(event OnComponentBeginOverlap(Box)
  (params (OverlappedComponent :type Primitive%20Component%20Object%20Reference) (OtherActor :type Actor%20Object%20Reference) (OtherComp :type Primitive%20Component%20Object%20Reference) (OtherBodyIndex :type Integer) (bFromSweep :type Boolean) (SweepResult :type Hit%20Result%20Structure%20%28by%20ref%29))
  ;[1 1 1] Door
  (Utilities|Casting|CastToBP_ThirdPersonCharacter OtherActor)
  (if (Variables|Default|GetDoor%20Unlocked)
    (Game|OpenLevel(byName) (Variables|Default|GetTargetLevelName))))

(event OnComponentBeginOverlap(Box1)
  (params (OverlappedComponent :type Primitive%20Component%20Object%20Reference) (OtherActor :type Actor%20Object%20Reference) (OtherComp :type Primitive%20Component%20Object%20Reference) (OtherBodyIndex :type Integer) (bFromSweep :type Boolean) (SweepResult :type Hit%20Result%20Structure%20%28by%20ref%29))
  (bind _supergrid_plane (Variables|Default|GetSuperGrid_Plane))
  (bind _supergrid_plane1 (Variables|Default|GetSuperGrid_Plane1))
  ;[1 1 1] Pressure Plate
  (Utilities|Casting|CastToBP_ThirdPersonCharacter OtherActor)
  (Variables|Default|SetPressure%20Plate%20Pressed true)
  (if (Variables|Default|GetPressure%20Plate%20Pressed)
    (Rendering|SetVisibility _supergrid_plane false false)
    (Collision|SetCollisionEnabled _supergrid_plane "NoCollision")
    (Rendering|SetVisibility _supergrid_plane1 false false)
    (Collision|SetCollisionEnabled _supergrid_plane1 "NoCollision")))

(event EventBeginPlay)

(event EventTick
  (params (DeltaSeconds :type Float%20%28single-precision%29)))

(fn ConstructionScript)